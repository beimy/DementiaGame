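; MedGearMove_BP is a gear actor that spins its DefaultSceneRoot1 component every Tick.
; Prioritized booleans pick one motion: CWVert lowers roll, CWHorz lowers yaw, CCVertical raises pitch, CCHorz raises yaw.
; CCHorz builds on actor rotation, while the other modes use the component's world rotation.
; RotationSpeed is applied per frame without delta-time scaling, so speed depends on frame rate.
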(event `self.ReceiveTick`
  (params (DeltaSeconds :type "Float (single-precision)"))
  (bind (_rotation_roll _rotation_pitch _rotation_yaw) (`KismetMathLibrary.BreakRotator` (`self.Rotation`)))
  (bind (_rotation_roll_2 _rotation_pitch_2 _rotation_yaw_2) (`KismetMathLibrary.BreakRotator` (`self.Rotation`)))
  (bind (_rotation_roll_3 _rotation_pitch_3 _rotation_yaw_3) (`KismetMathLibrary.BreakRotator` (`self.Rotation`)))
  (set `self.Rotation` (`SceneComponent.K2_GetComponentRotation` (`self.DefaultSceneRoot1`)))
  (if (`self.CW_Vert`)
    (`SceneComponent.K2_SetWorldRotation` (`self.DefaultSceneRoot1`) (`KismetMathLibrary.MakeRotator` (- _rotation_roll (`self.Rotation_Speed`)) _rotation_pitch _rotation_yaw) false false)
    (elif (`self.CW_Horz`)
      (`SceneComponent.K2_SetWorldRotation` (`self.DefaultSceneRoot1`) (`KismetMathLibrary.MakeRotator` _rotation_roll_3 _rotation_pitch_3 (- _rotation_yaw_3 (`self.Rotation_Speed`))) false false)
      (elif (`self.CC_Vertical`)
        (`SceneComponent.K2_SetWorldRotation` (`self.DefaultSceneRoot1`) (`KismetMathLibrary.MakeRotator` _rotation_roll_2 (+ _rotation_pitch_2 (`self.Rotation_Speed`)) _rotation_yaw_2) false false)
        (elif (`self.CC_Horz`)
          (`SceneComponent.K2_SetWorldRotation` (`self.DefaultSceneRoot1`) (`KismetMathLibrary.MakeRotator` (.roll (`self.K2_GetActorRotation`)) (.pitch (`self.K2_GetActorRotation`)) (+ (.yaw (`self.K2_GetActorRotation`)) (`self.Rotation_Speed`))) false false))))))

(fn `UserConstructionScript`)