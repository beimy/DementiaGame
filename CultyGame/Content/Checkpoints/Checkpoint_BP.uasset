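; Checkpoint actor that records or clears the player's respawn data when its box is overlapped, depending on its Load flag.
; With Load set, it writes the player character's location and a true Load flag to a Save_Point in slot "check", creating it if absent, then destroys itself after a delay.
; Otherwise it sets the saved Load flag to false.
; The overlapping actor is never checked.
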(event `self.Box.OnComponentBeginOverlap`
  (params (OverlappedComponent :type "PrimitiveComponent Object Reference") (OtherActor :type "Actor Object Reference") (OtherComp :type "PrimitiveComponent Object Reference") (OtherBodyIndex :type Integer) (bFromSweep :type Boolean) (SweepResult :type "HitResult Structure (by ref)"))
  (bind _playerloc (`self.PlayerLoc`))
  (if (`self.Load?`)
    (`|ExecutionSequence`
      (:`then_0`
        (bind _asthird_person_character (cast `/Game/ThirdPersonCPP/Blueprints/ThirdPersonCharacter` (`GameplayStatics.GetPlayerCharacter` 0)))
        (set `self.PlayerLoc` (`self.K2_GetActorLocation` _asthird_person_character))
        (`KismetSystemLibrary.PrintString` "Checkpoint Reached!"))
      (:`then_1`
        (bind _returnvalue (`GameplayStatics.DoesSaveGameExist` "check"))
        (if _returnvalue
          (bind _returnvalue_2 (`GameplayStatics.LoadGameFromSlot` "check"))
          (bind _assave_point (cast `/Game/Checkpoints/Save_Point` _returnvalue_2))
          (set `/Game/Checkpoints/Save_Point.PlayerLoc_s` _playerloc _assave_point)
          (set `/Game/Checkpoints/Save_Point.Load?` true _assave_point)
          (`GameplayStatics.SaveGameToSlot` _assave_point "check")
          (else
            (bind _returnvalue_3 (`GameplayStatics.CreateSaveGameObject` "/Game/Checkpoints/Save_Point.Save_Point_C"))
            (set `/Game/Checkpoints/Save_Point.PlayerLoc_s` _playerloc _returnvalue_3)
            (set `/Game/Checkpoints/Save_Point.Load?` true _returnvalue_3)
            (`GameplayStatics.SaveGameToSlot` _returnvalue_3 "check")))
        (`KismetSystemLibrary.Delay` 2.0)
        (`self.K2_DestroyActor`)))
    (else
      (bind _returnvalue_4 (`GameplayStatics.LoadGameFromSlot` "check"))
      (bind _assave_point_2 (cast `/Game/Checkpoints/Save_Point` _returnvalue_4))
      (set `/Game/Checkpoints/Save_Point.Load?` false _assave_point_2)
      (`GameplayStatics.SaveGameToSlot` _assave_point_2 "check")
      (`KismetSystemLibrary.PrintString` "Checkpoint Cleared!"))))

(fn `UserConstructionScript`)