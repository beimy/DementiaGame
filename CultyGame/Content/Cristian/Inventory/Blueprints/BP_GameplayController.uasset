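; Gameplay controller that handles the OpenInventory input and owns a reference to the player's inventory widget.
; On press, it re-adds the widget cached on ThirdPersonCharacter_BP to the viewport if valid.
; Otherwise it creates WB_Inventory, passes the character's Distract, Invisibility and Fire spell flags to InvSpellCheck, and caches the result on itself and the character.
; ReloadInventory tells the controller's cached widget to reload its items.
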(event `InputAction|OpenInventory`
  (params (Key :type "Key Structure"))
  (bind _playercontroller (`self.PlayerController`))
  ;[1 1 1] Open the player's inventory when the input action is received.
  (:`Pressed`
    (bind _asthird_person_character_bp (cast `/Game/ThirdPersonCPP/Blueprints/ThirdPersonCharacter_BP` (`GameplayStatics.GetPlayerCharacter` 0)))
    (bind _output_get (set `self.PlayerController` _asthird_person_character_bp))
    (bind _myinventorywidget (`/Game/ThirdPersonCPP/Blueprints/ThirdPersonCharacter_BP.MyInventoryWidget` _output_get))
    (`/Engine/EditorBlueprintResources/StandardMacros.IsValid` _myinventorywidget
      (:`Is Valid`
        (`UserWidget.AddToViewport` _myinventorywidget 0))
      (:`Is Not Valid`
        (bind _returnvalue (`|CreateWidget` "/Game/Cristian/Inventory/UI/WB_Inventory.WB_Inventory_C" (`GameplayStatics.GetPlayerController` 0)))
        (bind _myinventory (`/Game/Cristian/Inventory/UI/WB_Inventory.Inv_SpellCheck` _returnvalue (`/Game/ThirdPersonCPP/Blueprints/ThirdPersonCharacter_BP.DistractChk` _playercontroller) (`/Game/ThirdPersonCPP/Blueprints/ThirdPersonCharacter_BP.InvisiblityChk` _playercontroller) (`/Game/ThirdPersonCPP/Blueprints/ThirdPersonCharacter_BP.FireChk` _playercontroller)))
        (bind _output_get_2 (set `self.Inventory_Widget` _myinventory))
        (set `/Game/ThirdPersonCPP/Blueprints/ThirdPersonCharacter_BP.MyInventoryWidget` _output_get_2 (`self.PlayerController`))))))

(event `self.ReloadInventory`
  (bind _inventory_widget (`self.Inventory_Widget`))
  (`/Engine/EditorBlueprintResources/StandardMacros.IsValid` _inventory_widget
    (:`Is Valid`
      (`/Game/Cristian/Inventory/UI/WB_Inventory.LoadInventoryItems` _inventory_widget))))

(fn `UserConstructionScript`)