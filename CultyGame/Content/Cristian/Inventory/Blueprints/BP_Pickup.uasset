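; BP_Pickup is an interactable world pickup that adds an item to the player's inventory by ItemID.
; On Interact it plays an attached sound, passes non-spell items to BP_GameplayController, calls OnPickedUp and destroys itself.
; An optional linked tutorial trigger has collision disabled at BeginPlay and enabled on pickup; the HasTutorial check is disconnected.
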(event `self.Interact`
  (params (Controller :type "PlayerController Object Reference"))
  ;[1 1 1] On Interact, add interactable item to inventory.
  (if true
    (`GameplayStatics.SpawnSoundAttached` null null "None" (0.0 0.0 0.0) (struct) "KeepRelativeOffset" false 1.0 1.0 0.0 null null)
    (if (not (`self.IsSpell`))
      (`GameplayController.AddItemToInventoryByID` (cast `/Game/Cristian/Inventory/Blueprints/BP_GameplayController` Controller :!pure true) (`self.ItemID`)))
    (`self.OnPickedUp`)
    (`/Engine/EditorBlueprintResources/StandardMacros.IsValid` (`self.MyTutorialTrigger`)
      (:`Is Valid`
        ;[1 1 1] Check to trigger tutorial
        (`self.SetActorEnableCollision` (`self.MyTutorialTrigger`) true))
      (:`Is Not Valid`
        _))
    (`self.K2_DestroyActor`)))

(event `self.ReceiveBeginPlay`
  (`self.SetActorEnableCollision` (`self.MyTutorialTrigger`) false))

(fn `UserConstructionScript`)