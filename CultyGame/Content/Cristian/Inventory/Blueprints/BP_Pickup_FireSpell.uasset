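; Fire spell pickup in the inventory system that makes Fire the player's current spell when used.
; On the OnUsed event it casts the first player's pawn to ThirdPersonCharacter_BP and sets its CurrentSpell to "Fire".
; It has no other active logic, as BeginPlay, overlap and Tick are disabled stubs and construction only calls the parent.
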(event `self.OnUsed`
  (set `/Game/ThirdPersonCPP/Blueprints/ThirdPersonCharacter_BP.CurrentSpell` "Fire" (cast `/Game/ThirdPersonCPP/Blueprints/ThirdPersonCharacter_BP` (`GameplayStatics.GetPlayerPawn` 0) :!pure true)))

(fn `UserConstructionScript`
  (`parent.UserConstructionScript`))