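; Health potion pickup Blueprint that adds a fixed amount of health to the player when used.
; OnUsed prints a debug string, casts the first player character to ThirdPersonCharacter_BP, then sets HealthCurre to Healthcurr plus that amount, with no clamp.
; The read and written variable names differ.
; DestroyActor is unconnected, so use does not destroy the actor, and the BeginPlay and overlap events are disabled.
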(event `self.OnUsed`
  ;[1 1 1] Setup Health gain here
  (`KismetSystemLibrary.PrintString` "Hello")
  (bind _asthird_person_character_bp (cast `/Game/ThirdPersonCPP/Blueprints/ThirdPersonCharacter_BP` (`GameplayStatics.GetPlayerCharacter` 0)))
  (set `/Game/ThirdPersonCPP/Blueprints/ThirdPersonCharacter_BP.HealthCurre` (+ (`/Game/ThirdPersonCPP/Blueprints/ThirdPersonCharacter.healthcurr` _asthird_person_character_bp) 50.0) _asthird_person_character_bp))

(fn `UserConstructionScript`
  (`parent.UserConstructionScript`))