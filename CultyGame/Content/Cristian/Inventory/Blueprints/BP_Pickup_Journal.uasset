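; Journal pickup actor that opens a journal UI for the player when used.
; OnUsed casts the player pawn to ThirdPersonCharacter_BP and casts its own Journal variable to the Journal widget class.
; It then creates that widget for the first player controller, stores it on the character's Journal variable and adds it to the viewport.
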(event `self.OnUsed`
  (bind _asthird_person_character_bp (cast `/Game/ThirdPersonCPP/Blueprints/ThirdPersonCharacter_BP` (`GameplayStatics.GetPlayerPawn` 0)))
  (bind _asjournal (castclass `/Game/Widgets/Menus/Journal` "/Game/Widgets/Menus/Journal.Journal_C"))
  (bind _returnvalue (`|CreateWidget` _asjournal (`GameplayStatics.GetPlayerController` 0)))
  (bind _output_get (set `/Game/ThirdPersonCPP/Blueprints/ThirdPersonCharacter_BP.Journal` _returnvalue _asthird_person_character_bp))
  (`UserWidget.AddToViewport` _output_get 0))

(fn `UserConstructionScript`
  (`parent.UserConstructionScript`))