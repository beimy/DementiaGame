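; Talisman pickup that grants the player a spell when picked up.
; On BeginPlay it binds to its OnPickedUp event, then passes its Spell to the player character's inventory widget.
; It also tells the NPC manager about the pickup, has the character show a new-spell message, and destroys every actor in its Dependents list.
; The NewSpellGained function is a stub that returns an empty string.
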(event `self.ReceiveBeginPlay`
  (`parent.ReceiveBeginPlay`)
  (add `self.OnPickedUp` (delegate `PickupGrabbed`)))

(event `PickupGrabbed`
  (bind _asthird_person_character_bp (cast `/Game/ThirdPersonCPP/Blueprints/ThirdPersonCharacter_BP` (`GameplayStatics.GetPlayerCharacter` 0)))
  (`/Game/Cristian/Inventory/UI/WB_Inventory.GetSpell` (`/Game/ThirdPersonCPP/Blueprints/ThirdPersonCharacter_BP.MyInventoryWidget` _asthird_person_character_bp) (`self.Spell`))
  (message `/Game/Interactables/INF_Talisman_Manager.PickedUp` (`self.MyNPCManager`))
  (message `/Game/Interactables/INF_Talisman_Manager.NewSpell` _asthird_person_character_bp (`self.Spell`))
  (for _array_element (`self.Dependents`)
    (`self.K2_DestroyActor` _array_element)))

(fn `NewSpellGained`
  (params (SpellGive :type String))
  (returns (SpellTake :type String))
  (return ""))

(fn `UserConstructionScript`
  (`parent.UserConstructionScript`))