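; Crystal actor for the Jessebelle boss fight that can be damaged and destroyed.
; A C++ health component holds its health, which is printed on BeginPlay and whenever it takes damage.
; When damage finds health at zero or below, it casts its Boss reference to Jessebelle_Boss_Fight, increments that boss's DestroyedCrystals count and destroys itself.
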(event `self.ReceiveBeginPlay`
  ;[1 1 1] C++ Health Component
  (`KismetSystemLibrary.PrintString` (`KismetStringLibrary.Conv_DoubleToString` (`HealthComponent.Health` (`self.Health1`)))))

(event `self.ReceiveAnyDamage`
  (params (Damage :type "Float (single-precision)") (DamageType :type "DamageType Object Reference") (InstigatedBy :type "Controller Object Reference") (DamageCauser :type "Actor Object Reference"))
  ;[1 1 1] C++ Health Component
  (`KismetSystemLibrary.PrintString` (`KismetStringLibrary.Conv_DoubleToString` (`HealthComponent.Health` (`self.Health1`))))
  (if (<= (`HealthComponent.Health` (`self.Health1`)) 0.0)
    (`KismetSystemLibrary.PrintString` "Health IS 0.")
    (bind _asjessebelle_boss_fight (cast `/Game/Alberto/AI/Ai_2_YT/JesseBelle/Jessebelle_Boss_Fight` (`self.Boss`)))
    (bind _result (`/Engine/EditorBlueprintResources/StandardMacros.IncrementInt` (`/Game/Alberto/AI/Ai_2_YT/JesseBelle/Jessebelle_Boss_Fight.Destroyed Crystals` _asjessebelle_boss_fight))
      (:`  `
        (set `/Game/Alberto/AI/Ai_2_YT/JesseBelle/Jessebelle_Boss_Fight.Destroyed Crystals` _result _asjessebelle_boss_fight)
        (`self.K2_DestroyActor`)))
    (else
      (`KismetSystemLibrary.PrintString` "Health ISN'T 0."))))

(fn `UserConstructionScript`)