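; BP_DoorShed is a shed door that swings open when the third-person character enters its trigger box.
; Begin overlap registers the door as the character's Interactable, prints a debug message and plays the Doors timeline, which scales Angle to set the Scene component's relative yaw.
; End overlap only clears IsPlayer, with no closing motion.
; A button-press check on IsPlayer and PressedButton is left unconnected.
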(event `self.Box.OnComponentEndOverlap`
  (params (OverlappedComponent :type "PrimitiveComponent Object Reference") (OtherActor :type "Actor Object Reference") (OtherComp :type "PrimitiveComponent Object Reference") (OtherBodyIndex :type Integer))
  (cast `/Game/ThirdPersonCPP/Blueprints/ThirdPersonCharacter_BP` OtherActor)
  (set `self.IsPlayer` false))

(event `self.Box.OnComponentBeginOverlap`
  (params (OverlappedComponent :type "PrimitiveComponent Object Reference") (OtherActor :type "Actor Object Reference") (OtherComp :type "PrimitiveComponent Object Reference") (OtherBodyIndex :type Integer) (bFromSweep :type Boolean) (SweepResult :type "HitResult Structure (by ref)"))
  (bind _asthird_person_character_bp (cast `/Game/ThirdPersonCPP/Blueprints/ThirdPersonCharacter_BP` OtherActor))
  (set `/Game/ThirdPersonCPP/Blueprints/ThirdPersonCharacter_BP.Interactable` self _asthird_person_character_bp)
  (`KismetSystemLibrary.PrintString` "Interactable set")
  (bind (_direction _newtrack_0) (`Timeline|Doors`)
    (:`Update`
      (`SceneComponent.K2_SetRelativeRotation` (`self.Scene`) (`KismetMathLibrary.MakeRotator` 0.0 0.0 (* _newtrack_0 (`self.Angle`))) false false))))

(fn `UserConstructionScript`)