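; MadnessFog_BP is a fog hazard that raises the player character's madness while it stands inside the DamageRadi volume.
; Beginning overlap with a ThirdPersonCharacter_BP stores it and sets InField, starting a Delay-based loop that calls IncreaseMadness every half second.
; Any end overlap on the volume clears InField, regardless of actor, which stops the loop.
; The DamageTick function only checks InField and has no effect.
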(event `self.DamageRadi.OnComponentBeginOverlap`
  (params (OverlappedComponent :type "PrimitiveComponent Object Reference") (OtherActor :type "Actor Object Reference") (OtherComp :type "PrimitiveComponent Object Reference") (OtherBodyIndex :type Integer) (bFromSweep :type Boolean) (SweepResult :type "HitResult Structure (by ref)"))
  (bind _asthird_person_character_bp (cast `/Game/ThirdPersonCPP/Blueprints/ThirdPersonCharacter_BP` OtherActor))
  (set `self.PC` _asthird_person_character_bp)
  (set `self.InField` true)
  (if (`self.InField`) :!label _label
    (`/Game/ThirdPersonCPP/Blueprints/ThirdPersonCharacter_BP.IncreaseMadness` (`self.PC`) 10.0)
    (`KismetSystemLibrary.Delay` 0.5)
    (goto _label)))

(event `self.DamageRadi.OnComponentEndOverlap`
  (params (OverlappedComponent :type "PrimitiveComponent Object Reference") (OtherActor :type "Actor Object Reference") (OtherComp :type "PrimitiveComponent Object Reference") (OtherBodyIndex :type Integer))
  (set `self.InField` false))

(fn `DamageTick`
  (if (`self.InField`)
    _))

(fn `UserConstructionScript`)